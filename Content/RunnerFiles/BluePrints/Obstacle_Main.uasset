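; Runner obstacle Blueprint that kills the player on contact and rewards close dodges with brief slow motion.
; The Death volume calls DeathF on the overlapping PawnCharacters, while Front flags IsFrontCloseDodge.
; Middle clears that flag and triggers SlowMotionF if it was set; Back triggers SlowMotionF when it is unset.
; After a short delay, both restore global time dilation, clear all widgets and recreate InGameUI.
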(event `self.ReceiveActorBeginOverlap`
  (params (OtherActor :type "Actor Object Reference")))

(event `self.Death.OnComponentBeginOverlap`
  (params (OverlappedComponent :type "PrimitiveComponent Object Reference") (OtherActor :type "Actor Object Reference") (OtherComp :type "PrimitiveComponent Object Reference") (OtherBodyIndex :type Integer) (bFromSweep :type Boolean) (SweepResult :type "HitResult Structure (by ref)"))
  (bind _aspawn_characters (cast `/Game/ThirdPerson/Blueprints/PawnCharacters` OtherActor))
  (`/Game/ThirdPerson/Blueprints/PawnCharacters.Death F` _aspawn_characters))

(event `self.Back.OnComponentBeginOverlap`
  (params (OverlappedComponent :type "PrimitiveComponent Object Reference") (OtherActor :type "Actor Object Reference") (OtherComp :type "PrimitiveComponent Object Reference") (OtherBodyIndex :type Integer) (bFromSweep :type Boolean) (SweepResult :type "HitResult Structure (by ref)"))
  (bind _aspawn_characters (cast `/Game/ThirdPerson/Blueprints/PawnCharacters` OtherActor))
  (if (not (`/Game/ThirdPerson/Blueprints/PawnCharacters.IsFrontCloseDodge` _aspawn_characters))
    (`/Game/ThirdPerson/Blueprints/PawnCharacters.SlowMotionF` _aspawn_characters)
    (`KismetSystemLibrary.Delay` 0.5)
    (`WidgetLayoutLibrary.RemoveAllWidgets`)
    (`GameplayStatics.SetGlobalTimeDilation` 1.0)
    (bind _returnvalue (`|CreateWidget` "/Game/RunnerFiles/UI/InGameUI.InGameUI_C"))
    (`UserWidget.AddToViewport` _returnvalue 0)))

(event `self.Middle.OnComponentBeginOverlap`
  (params (OverlappedComponent :type "PrimitiveComponent Object Reference") (OtherActor :type "Actor Object Reference") (OtherComp :type "PrimitiveComponent Object Reference") (OtherBodyIndex :type Integer) (bFromSweep :type Boolean) (SweepResult :type "HitResult Structure (by ref)"))
  (bind _aspawn_characters (cast `/Game/ThirdPerson/Blueprints/PawnCharacters` OtherActor))
  (if (`/Game/ThirdPerson/Blueprints/PawnCharacters.IsFrontCloseDodge` _aspawn_characters)
    (set `/Game/ThirdPerson/Blueprints/PawnCharacters.IsFrontCloseDodge` false _aspawn_characters)
    (`/Game/ThirdPerson/Blueprints/PawnCharacters.SlowMotionF` _aspawn_characters)
    (`KismetSystemLibrary.Delay` 0.5)
    (`WidgetLayoutLibrary.RemoveAllWidgets`)
    (`GameplayStatics.SetGlobalTimeDilation` 1.0)
    (bind _returnvalue (`|CreateWidget` "/Game/RunnerFiles/UI/InGameUI.InGameUI_C"))
    (`UserWidget.AddToViewport` _returnvalue 0)))

(event `self.Front.OnComponentBeginOverlap`
  (params (OverlappedComponent :type "PrimitiveComponent Object Reference") (OtherActor :type "Actor Object Reference") (OtherComp :type "PrimitiveComponent Object Reference") (OtherBodyIndex :type Integer) (bFromSweep :type Boolean) (SweepResult :type "HitResult Structure (by ref)"))
  (bind _aspawn_characters (cast `/Game/ThirdPerson/Blueprints/PawnCharacters` OtherActor))
  (set `/Game/ThirdPerson/Blueprints/PawnCharacters.IsFrontCloseDodge` true _aspawn_characters)
  (`KismetSystemLibrary.PrintString` (`KismetStringLibrary.Conv_BoolToString` false)))

(fn `UserConstructionScript`)