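; Runner pawn holding two characters, Left and Right capsules, that each switch between two lanes by keys or touch buttons.
; BeginPlay takes lane locations from EndlessTile, and per-side timelines lerp each capsule between them.
; Right-side switches check CanSwitchRight but toggle CanSwitchLeft.
; DeathF pauses, shows GameOver and saves the game mode's score as high score, while SlowMotionF halves time dilation and shows a CloseDodge widget.
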(event `self.ReceiveTick`
  (params (DeltaSeconds :type "Float (single-precision)")))

(event `Key|A`
  (params (Key :type "Key Structure"))
  (bind _leftlanelocation (`self.LeftLaneLocation`))
  (bind _leftcapsule (`self.LeftCapsule`))
  ;[0.3476 0.4402 1] LeftCharacter
  (:`Pressed`
    (if (`self.CanSwitchLeft`) :!label _label
      (set `self.CanSwitchLeft` false)
      (set `self.NewLeftLane` (`KismetMathLibrary.Clamp` (+ (`self.LeftLane`) 1) 0 1))
      (bind (_direction _track) (`Timeline|Timeline` :!via `PlayFromStart` :!label _label_2)
        (:`Update`
          (bind (_returnvalue_x _returnvalue_y _returnvalue_z) (`KismetMathLibrary.BreakVector` (`KismetMathLibrary.VLerp` (`|GetArrayItem` _leftlanelocation (`self.LeftLane`)) (`|GetArrayItem` _leftlanelocation (`self.NewLeftLane`)) _track)))
          (`SceneComponent.K2_SetWorldLocation` _leftcapsule (`KismetMathLibrary.MakeVector` _returnvalue_x _returnvalue_y (+ _returnvalue_z (`CapsuleComponent.GetScaledCapsuleHalfHeight` _leftcapsule))) false false))
        (:`Finished`
          (set `self.CanSwitchLeft` true)
          (set `self.LeftLane` (`self.NewLeftLane`)))))))

(event `LeftTouchButton`
  (if (== (`self.LeftLane`) 0)
    (goto _label)
    (else
      ;[0.3476 0.4402 1] LeftCharacter
      (if (`self.CanSwitchLeft`) :!label _label_3
        (set `self.CanSwitchLeft` false)
        (set `self.NewLeftLane` (`KismetMathLibrary.Clamp` (+ (`self.LeftLane`) -1) 0 1))
        (goto _label_2 :!via `PlayFromStart`)))))

(event `Key|D`
  (params (Key :type "Key Structure"))
  ;[0.3476 0.4402 1] LeftCharacter
  (:`Pressed`
    (goto _label_3)))

(event `self.ReceiveBeginPlay`
  (bind _leftcapsule (`self.LeftCapsule`))
  (bind _rightcapsule (`self.RightCapsule`))
  (bind (_output_x _output_y _output_z) (`KismetMathLibrary.BreakVector` (`|GetArrayItem` (`self.RightLaneLocation`) (`self.RightLane`))))
  (bind (_output_x_2 _output_y_2 _output_z_2) (`KismetMathLibrary.BreakVector` (`|GetArrayItem` (`self.LeftLaneLocation`) (`self.LeftLane`))))
  (bind _returnvalue (`GameplayStatics.GetActorOfClass` "/Game/RunnerFiles/BluePrints/EndlessTile.EndlessTile_C"))
  (set `self.LeftLaneLocation` (`/Game/RunnerFiles/BluePrints/EndlessTile.LeftLaneLocations` _returnvalue))
  (set `self.RightLaneLocation` (`/Game/RunnerFiles/BluePrints/EndlessTile.RightLaneLocations` _returnvalue))
  (bind (_returnvalue_x _returnvalue_y _returnvalue_z) (`KismetMathLibrary.BreakVector` (`SceneComponent.K2_GetComponentLocation` (`/Game/RunnerFiles/BluePrints/EndlessTile.Center` _returnvalue))))
  (`self.K2_SetActorLocation` (`KismetMathLibrary.MakeVector` _returnvalue_x _returnvalue_y _returnvalue_z))
  (`SceneComponent.K2_SetWorldLocation` _rightcapsule (`KismetMathLibrary.MakeVector` _output_x _output_y (+ _output_z (`CapsuleComponent.GetScaledCapsuleHalfHeight` _rightcapsule))) false false)
  (`SceneComponent.K2_SetWorldLocation` _leftcapsule (`KismetMathLibrary.MakeVector` _output_x_2 _output_y_2 (+ _output_z_2 (`CapsuleComponent.GetScaledCapsuleHalfHeight` _leftcapsule))) false false))

(event `Key|R`
  (params (Key :type "Key Structure")))

(event `resetdoonceright`
  ;[0.3476 0.4402 1] RightCharacter
  (`/Engine/EditorBlueprintResources/StandardMacros.DoOnce` false :!via `Reset`))

(event `Key|Right`
  (params (Key :type "Key Structure"))
  (bind _rightlanelocation (`self.RightLaneLocation`))
  (bind _rightcapsule (`self.RightCapsule`))
  ;[0.3476 0.4402 1] RightCharacter
  (:`Pressed`
    (if (`self.CanSwitchRight`) :!label _label_4
      (set `self.CanSwitchLeft` false)
      (set `self.NewRightLane` (`KismetMathLibrary.Clamp` (+ (`self.RightLane`) 1) 0 1))
      (bind (_direction _track) (`Timeline|Timeline_0` :!via `PlayFromStart` :!label _label_5)
        (:`Update`
          (bind (_returnvalue_x _returnvalue_y _returnvalue_z) (`KismetMathLibrary.BreakVector` (`KismetMathLibrary.VLerp` (`|GetArrayItem` _rightlanelocation (`self.RightLane`)) (`|GetArrayItem` _rightlanelocation (`self.NewRightLane`)) _track)))
          (`SceneComponent.K2_SetWorldLocation` _rightcapsule (`KismetMathLibrary.MakeVector` _returnvalue_x _returnvalue_y (+ _returnvalue_z (`CapsuleComponent.GetScaledCapsuleHalfHeight` _rightcapsule))) false false))
        (:`Finished`
          (set `self.CanSwitchLeft` true)
          (set `self.RightLane` (`self.NewRightLane`)))))))

(event `RightTouchButton`
  (if (== (`self.RightLane`) 0)
    (goto _label_4)
    (else
      ;[0.3476 0.4402 1] RightCharacter
      (if (`self.CanSwitchRight`) :!label _label_6
        (set `self.CanSwitchLeft` false)
        (set `self.NewRightLane` (`KismetMathLibrary.Clamp` (+ (`self.RightLane`) -1) 0 1))
        (goto _label_5 :!via `PlayFromStart`)))))

(event `Key|Left`
  (params (Key :type "Key Structure"))
  ;[0.3476 0.4402 1] RightCharacter
  (:`Pressed`
    (goto _label_6)))

(fn `Death F`
  (bind _savesubclass (`self.SaveSubClass`))
  (`GameplayStatics.SetGamePaused` true)
  (bind _returnvalue (`|CreateWidget` "/Game/RunnerFiles/UI/GameOver.GameOver_C"))
  (`UserWidget.AddToViewport` _returnvalue 0)
  (bind _asbp_third_person_game_mode (cast `/Game/RunnerFiles/BluePrints/BP_ThirdPersonGameMode` (`GameplayStatics.GetGameMode`)))
  (bind _returnvalue_2 (`GameplayStatics.DoesSaveGameExist` "HighScore"))
  (if _returnvalue_2
    (bind _returnvalue_3 (`GameplayStatics.LoadGameFromSlot` "HighScore"))
    (bind _output_get (set `self.SaveSubClass` _returnvalue_3))
    (bind _asscore_save (cast `/Game/RunnerFiles/BluePrints/ScoreSave` _output_get))
    (bind _currentscore (`/Game/RunnerFiles/BluePrints/BP_ThirdPersonGameMode.CurrentScore` _asbp_third_person_game_mode))
    (if (> _currentscore (`/Game/RunnerFiles/BluePrints/ScoreSave.HighScoreValue` _asscore_save))
      (set `/Game/RunnerFiles/BluePrints/ScoreSave.HighScoreValue` _currentscore _asscore_save)
      (`GameplayStatics.SaveGameToSlot` _savesubclass "HighScore"))
    (else
      (bind _returnvalue_4 (`GameplayStatics.CreateSaveGameObject` "/Game/RunnerFiles/BluePrints/ScoreSave.ScoreSave_C"))
      (bind _output_get_2 (set `self.SaveSubClass` _returnvalue_4))
      (bind _asscore_save_2 (cast `/Game/RunnerFiles/BluePrints/ScoreSave` _output_get_2))
      (set `/Game/RunnerFiles/BluePrints/ScoreSave.HighScoreValue` _currentscore _asscore_save_2)
      (`GameplayStatics.SaveGameToSlot` _savesubclass "HighScore"))))

(fn `SlowMotionF`
  (`GameplayStatics.SetGlobalTimeDilation` 0.5)
  (bind _returnvalue (`|CreateWidget` "/Game/RunnerFiles/UI/CloseDodge.CloseDodge_C"))
  (`UserWidget.AddToViewport` _returnvalue 0))

(fn `UserConstructionScript`)